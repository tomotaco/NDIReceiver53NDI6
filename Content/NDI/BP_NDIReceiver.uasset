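; BP_NDIReceiver is a Blueprint that receives an NDI stream and plays it on a plane with a media sound output.
; On BeginPlay it opens the MS_NDIReceiver media source in a MediaPlayer and connects the receiver to the source named by MediaSourceURL.
; It then creates a dynamic instance of ScreenMaterial on the Plane, feeds MediaTexture into its Texture parameter, and binds MediaSound to the player.
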(event EventBeginPlay
  (bind _returnvalue (Class|NDIIOLibrary|GetNDIMediaReceiver "/Game/NDI/MS_NDIReceiver.MS_NDIReceiver"))
  (Media|MediaPlayer|OpenSource (Variables|Default|GetMediaPlayer) _returnvalue)
  (Class|NDIMediaReceiver|ChangeConnection _returnvalue (Utilities|Struct|MakeNDIConnectionInformation (Variables|Default|GetMediaSourceURL)))
  (bind _returnvalue_2 (Rendering|Material|CreateDynamicMaterialInstance (Variables|Default|GetPlane) 0 (Variables|Default|GetScreenMaterial) "None" :!class /Script/Engine.PrimitiveComponent))
  (bind _output_get (Variables|Default|SetDynamicMaterial _returnvalue_2))
  (Rendering|Material|SetTextureParameterValue _output_get "Texture" (Variables|Default|GetMediaTexture))
  (Media|MediaSoundComponent|SetMediaPlayer (Variables|Default|GetMediaSound) (Variables|Default|GetMediaPlayer)))

(fn ConstructionScript)